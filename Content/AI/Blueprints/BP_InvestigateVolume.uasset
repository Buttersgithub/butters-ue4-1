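; BP_InvestigateVolume is an AI trigger volume that accumulates a suspicion score while the player is inside it.
; Box overlaps with BP_Player toggle PlayerInside, and a looping timer increments SuspicionAmount while that flag is set.
; The count never decreases here, and nothing in this Blueprint acts on it.
; A Debug flag shows a text label with the count, turned toward the player on Tick.
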(event OnComponentBeginOverlap(Box)
  (params (OverlappedComponent :type Primitive%20Component%20Object%20Reference) (OtherActor :type Actor%20Object%20Reference) (OtherComp :type Primitive%20Component%20Object%20Reference) (OtherBodyIndex :type Integer) (bFromSweep :type Boolean) (SweepResult :type Hit%20Result%20Structure%20%28by%20ref%29))
  ;[1 0.05729 0.05729] Overlapping
  (Utilities|Casting|CastToBP_Player OtherActor)
  (Variables|Default|SetbPlayerInside true))

(event OnComponentEndOverlap(Box)
  (params (OverlappedComponent :type Primitive%20Component%20Object%20Reference) (OtherActor :type Actor%20Object%20Reference) (OtherComp :type Primitive%20Component%20Object%20Reference) (OtherBodyIndex :type Integer))
  ;[1 0.05729 0.05729] Overlapping
  (Utilities|Casting|CastToBP_Player OtherActor)
  (Variables|Default|SetbPlayerInside false))

(event Custom|Increment
  ;[1 0.05729 0.05729] Begin Play /  Event
  (if (Variables|Default|GetbPlayerInside)
    (Math|Integer|IncrementInt (Variables|Default|GetSuspicion%20Amount))))

(event EventBeginPlay
  ;[1 0.05729 0.05729] Begin Play /  Event
  (Utilities|Time|SetTimerbyEvent (delegate Custom|Increment) (Variables|Default|GetTime) true))

(event EventTick
  (params (DeltaSeconds :type Float%20%28single-precision%29))
  ;[1 0.05729 0.05729] Tick
  (if (Variables|Default|GetbDebug)
    (Utilities|IsValid (CallFunction|GetPlayer)
      (:Is%20Valid
        (Transformation|SetWorldRotation (Variables|Default|GetTextRender) (Math|Rotator|MakeRotator 0.0 0.0 (.yaw (Math|Rotator|FindLookatRotation (Transformation|GetWorldLocation (Variables|Default|GetTextRender)) (Transformation|GetActorLocation (CallFunction|GetPlayer))))) false false)
        (Rendering|Components|TextRender|SetText (Variables|Default|GetTextRender) (Utilities|Text|ToText(String) (Utilities|String|Append (Utilities|GetDisplayName self) " 
Suspicion Amount: " (Utilities|String|ToString(Integer) (Variables|Default|GetSuspicion%20Amount)))))))))

(fn ConstructionScript
  (bind _textrender (Variables|Default|GetTextRender))
  (bind _textrender_2 (Variables|Default|GetTextRender))
  (bind _textrender_3 (Variables|Default|GetTextRender))
  (if (Variables|Default|GetbDebug)
    (Development|SetHiddeninGame _textrender_2 false false)
    (Rendering|SetVisibility _textrender_3 true false)
    (Transformation|SetWorldScale3D _textrender "2.000000,2.000000,2.000000")
    (Rendering|Components|TextRender|SetText (Variables|Default|GetTextRender) (Utilities|Text|ToText(String) (Utilities|String|Append (Utilities|GetDisplayName self) " 
Suspicion Amount: " (Utilities|String|ToString(Integer) (Variables|Default|GetSuspicion%20Amount)))))
    (else
      (Development|SetHiddeninGame _textrender_2 true false)
      (Rendering|SetVisibility _textrender_3 false false)
      (Transformation|SetWorldScale3D _textrender "2.000000,2.000000,20.000000"))))