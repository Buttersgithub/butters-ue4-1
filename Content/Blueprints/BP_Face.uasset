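; BP_Face is a stalker enemy Character that chases the player while unseen and jumpscares them on contact.
; Each tick it eases its capsule rotation toward the player, stops if recently rendered, and otherwise calls AIMoveTo on the player.
; Sphere overlap with FirstPersonCharacter starts a DoOnce-gated timeline that fades in post-processing, resets the gate after a delay, and finally sets control rotation from the Face component's relative rotation.
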(event OnComponentBeginOverlap(Sphere)
  (params (OverlappedComponent :type Primitive%20Component%20Object%20Reference) (OtherActor :type Actor%20Object%20Reference) (OtherComp :type Primitive%20Component%20Object%20Reference) (OtherBodyIndex :type Integer) (bFromSweep :type Boolean) (SweepResult :type Hit%20Result%20Structure%20%28by%20ref%29))
  ;[1 0.3785 0.901] Jumpscare
  (Utilities|Casting|CastToFirstPersonCharacter OtherActor)
  (Utilities|FlowControl|DoOnce false :!label _label
    (:Completed
      (bind _post_processing (Timeline|TL_Jumpscare PlayFromStart)
        (:Update
          (Variables|/Script/Engine.PostProcessComponent|SetBlendWeight (Variables|Default|GetPostProcess) (Math|Float|Lerp 0.0 1.0 _post_processing))
          (Utilities|FlowControl|Delay 2.0)
          (goto _label Reset))
        (:Finished
          (Pawn|SetControlRotation (Game|GetPlayerController 0) (Variables|/Script/Engine.SceneComponent|GetRelativeRotation (Variables|Default|GetFace))))))))

(event Custom|Face%20Player
  (bind _capsulecomponent (Variables|Collision|GetCapsuleComponent))
  ;[1 0.3785 0.901] Look at Player
  (Transformation|SetRelativeRotation _capsulecomponent (Math|Interpolation|Ease "EaseInOut" 0.25 (Variables|/Script/Engine.SceneComponent|GetRelativeRotation _capsulecomponent) (Math|Rotator|FindLookatRotation (Transformation|GetActorLocation) (Transformation|GetActorLocation (Game|GetPlayerCharacter 0))) true) false false))

(event Custom|Check%20if%20was%20recently%20Rendered
  ;[1 0.3785 0.901] AI
  (if (Class|Actor|WasRecentlyRendered 0.2)
    (Components|Movement|StopMovementImmediately (Variables|Character|GetCharacterMovement))
    (else
      (AI|AIMoveTo self "0, 0, 0" (Game|GetPlayerCharacter 0) 5.0 false))))

(event EventTick
  (params (DeltaSeconds :type Float%20%28single-precision%29))
  ;[1 0.3785 0.901] Tick
  (CallFunction|FacePlayer)
  (CallFunction|CheckifWasRecentlyRendered))

(fn ConstructionScript)