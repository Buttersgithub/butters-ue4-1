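; BP_Door is a door actor that swings open or closed about its yaw axis each time its OpenDoor event is called.
; A FlipFlop alternates between playing and reversing a timeline, whose output lerps the Door component's relative yaw from zero to the Rotation variable.
; The timeline play rate is the inverse of Speed, so Speed scales how long the swing takes.
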(event Custom|Open%20Door
  (bind _tl_door (Variables|Default|GetTL_Door))
  (bind _speed (Variables|Default|GetSpeed))
  (bind _returnvalue (/ 1.0 _speed))
  (Utilities|FlowControl|FlipFlop
    (:A
      (Components|Timeline|SetPlayRate _tl_door _returnvalue)
      (bind _rotation (Timeline|TL_Door Play)
        (:Update
          (Transformation|SetRelativeRotation (Variables|Default|GetDoor) (Math|Rotator|MakeRotator 0.0 0.0 (Math|Float|Lerp 0.0 (Variables|Default|GetRotation) _rotation)) false false))))
    (:B
      (Components|Timeline|SetPlayRate _tl_door _returnvalue)
      (Timeline|TL_Door Reverse))))

(event EventBeginPlay)

(fn ConstructionScript)