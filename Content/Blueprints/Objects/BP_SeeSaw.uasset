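; BP_SeeSaw is a seesaw object that launches the player character when its Cube tilts far enough.
; A looping timer from BeginPlay polls the Cube's pitch and, past a negative threshold, launches player 0 along the actor's up vector.
; Box overlaps with BP_Player toggle a PlayerRiding flag, but the launch check never reads it, so launching does not depend on riding.
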(event OnComponentBeginOverlap(Box)
  (params (OverlappedComponent :type Primitive%20Component%20Object%20Reference) (OtherActor :type Actor%20Object%20Reference) (OtherComp :type Primitive%20Component%20Object%20Reference) (OtherBodyIndex :type Integer) (bFromSweep :type Boolean) (SweepResult :type Hit%20Result%20Structure%20%28by%20ref%29))
  (Utilities|Casting|CastToBP_Player OtherActor)
  (Variables|Default|SetbPlayerRiding true))

(event OnComponentEndOverlap(Box)
  (params (OverlappedComponent :type Primitive%20Component%20Object%20Reference) (OtherActor :type Actor%20Object%20Reference) (OtherComp :type Primitive%20Component%20Object%20Reference) (OtherBodyIndex :type Integer))
  (Utilities|Casting|CastToBP_Player OtherActor)
  (Variables|Default|SetbPlayerRiding false))

(event Custom|Check%20Seesaw%20Velocity
  (if (<= (.pitch (Transformation|GetWorldRotation (Variables|Default|GetCube))) -1e+01)
    (Character|LaunchCharacter (Game|GetPlayerCharacter 0) (* (Transformation|GetActorUpVector) 5e+02) false false)))

(event EventBeginPlay
  (Utilities|Time|SetTimerbyEvent (delegate Custom|Check%20Seesaw%20Velocity) 0.1 true))

(fn ConstructionScript)