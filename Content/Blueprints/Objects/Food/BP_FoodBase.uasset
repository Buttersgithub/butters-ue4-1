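; Base food pickup that hungry BP_BaseOpponent actors eat to replenish hunger, with a random food value and material intensity set at BeginPlay.
; A box overlap feeds an opponent once if its hunger is low and CanEat is set, then a timeline shrinks the cube before destroying the actor.
; An optional debug text shows the actor name and CanEat state, turning each tick to face the player.
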(event OnComponentBeginOverlap(Box)
  (params (OverlappedComponent :type Primitive%20Component%20Object%20Reference) (OtherActor :type Actor%20Object%20Reference) (OtherComp :type Primitive%20Component%20Object%20Reference) (OtherBodyIndex :type Integer) (bFromSweep :type Boolean) (SweepResult :type Hit%20Result%20Structure%20%28by%20ref%29))
  ;[0 1 0.2291] Eat
  (bind _asbp_base_opponent (Utilities|Casting|CastToBP_BaseOpponent OtherActor))
  (if (and (<= (Variables|/Game/Characters/NPC/Opponent/BP_BaseOpponent.BP_BaseOpponent_C|GetHunger _asbp_base_opponent) 25.0) (Variables|Default|GetbCanEat))
    (Utilities|FlowControl|DoOnce false
      (:Completed
        (Default|ReplenishHunger _asbp_base_opponent (Variables|Default|GetHunger%20To%20Replenish))
        (bind _scale (Timeline|TL_Eaten PlayFromStart)
          (:Update
            (Transformation|SetRelativeScale3D (Variables|Default|GetCube) (Math|Vector|Lerp(Vector) "1.000000,1.000000,1.000000" "0, 0, 0" _scale)))
          (:Finished
            (Actor|DestroyActor)))))))

(event EventTick
  (params (DeltaSeconds :type Float%20%28single-precision%29))
  ;[0 1 0.2291] Tick
  (if (Variables|Default|GetbDebug)
    (Transformation|SetWorldRotation (Variables|Default|GetTextRender) (Math|Rotator|MakeRotator 0.0 0.0 (.yaw (Math|Rotator|FindLookatRotation (Transformation|GetWorldLocation (Variables|Default|GetTextRender)) (Transformation|GetActorLocation (Game|GetPlayerCharacter 0))))) false false)
    (Rendering|Components|TextRender|SetText (Variables|Default|GetTextRender) (Utilities|Text|ToText(String) (Utilities|String|Append (Utilities|GetDisplayName self) " 
Selected:  " (Utilities|String|ToString(Boolean) (Variables|Default|GetbCanEat)))))))

(event EventBeginPlay
  ;[0 1 0.2291] Begin Play
  (Rendering|Material|SetScalarParameterValueonMaterials (Variables|Default|GetCube) "Intensity" (Math|Random|RandomFloatinRange 2.0 1e+01))
  (Variables|Default|SetHunger%20To%20Replenish (Math|Random|RandomFloatinRange 5e+01 1e+02)))

(fn ConstructionScript
  (bind _textrender (Variables|Default|GetTextRender))
  (bind _textrender_2 (Variables|Default|GetTextRender))
  (if (Variables|Default|GetbDebug)
    (Rendering|SetVisibility _textrender true false)
    (Development|SetHiddeninGame _textrender_2 false false)
    (else
      (Rendering|SetVisibility _textrender false false)
      (Development|SetHiddeninGame _textrender_2 true false)))
  (Rendering|Components|TextRender|SetText (Variables|Default|GetTextRender) (Utilities|Text|ToText(String) (Utilities|String|Append (Utilities|GetDisplayName self) " 
Selected:  " (Utilities|String|ToString(Boolean) (Variables|Default|GetbCanEat))))))