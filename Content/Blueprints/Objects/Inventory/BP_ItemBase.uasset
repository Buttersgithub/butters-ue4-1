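; BP_ItemBase is the base inventory item actor, with pickup, drop and empty Use and SetObjectPosition functions.
; Pickup and Drop toggle mesh physics and collision, with Pickup also playing a sound and repeating its logic in a server event.
; The first angry BP_BaseOpponent overlapping the box picks up and attaches the item, clearing its anger.
; Any mesh hit on an opponent kills it with a forward impulse.
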(event OnComponentBeginOverlap(Box)
  (params (OverlappedComponent :type Primitive%20Component%20Object%20Reference) (OtherActor :type Actor%20Object%20Reference) (OtherComp :type Primitive%20Component%20Object%20Reference) (OtherBodyIndex :type Integer) (bFromSweep :type Boolean) (SweepResult :type Hit%20Result%20Structure%20%28by%20ref%29))
  (bind _asbp_base_opponent (Utilities|Casting|CastToBP_BaseOpponent OtherActor))
  (if (Variables|/Game/Characters/NPC/Opponent/BP_BaseOpponent.BP_BaseOpponent_C|GetbAngry _asbp_base_opponent)
    (Utilities|FlowControl|DoOnce false
      (:Completed
        (CallFunction|Pickup)
        (Transformation|AttachComponentToComponent self (Variables|/Game/Characters/NPC/Opponent/BP_BaseOpponent.BP_BaseOpponent_C|GetObject _asbp_base_opponent) "None" "SnapToTarget" "SnapToTarget" "KeepWorld" true)
        (Variables|/Game/Characters/NPC/Opponent/BP_BaseOpponent.BP_BaseOpponent_C|SetAnger _asbp_base_opponent 0.0)
        (Variables|/Game/Characters/NPC/Opponent/BP_BaseOpponent.BP_BaseOpponent_C|SetbAngry _asbp_base_opponent false)))))

(event OnComponentHit(StaticMesh)
  (params (HitComponent :type Primitive%20Component%20Object%20Reference) (OtherActor :type Actor%20Object%20Reference) (OtherComp :type Primitive%20Component%20Object%20Reference) (NormalImpulse :type Vector :default "0, 0, 0") (Hit :type Hit%20Result%20Structure%20%28by%20ref%29))
  (bind _asbp_base_opponent (Utilities|Casting|CastToBP_BaseOpponent OtherActor))
  (Variables|/Game/Characters/NPC/Opponent/BP_BaseOpponent.BP_BaseOpponent_C|SetbAlive _asbp_base_opponent false)
  (Default|Kill _asbp_base_opponent true true (* (Transformation|GetActorForwardVector) 2e+04)))

(event Custom|Pickup%20%28Server%29
  (bind _staticmesh (Variables|Default|GetStaticMesh))
  (Physics|SetSimulatePhysics _staticmesh false)
  (Collision|SetCollisionEnabled _staticmesh "NoCollision")
  (Audio|PlaySoundatLocation (Variables|Default|GetPickup%20Sound) (Transformation|GetActorLocation) "0, 0, 0" 1.0 1.0 0.0 0 0 0)
  (Variables|Default|SetbPickedUp true))

(fn ConstructionScript)

(fn Pickup
  (bind _staticmesh (Variables|Default|GetStaticMesh))
  (Physics|SetSimulatePhysics _staticmesh false)
  (Collision|SetCollisionEnabled _staticmesh "NoCollision")
  (Audio|PlaySoundatLocation (Variables|Default|GetPickup%20Sound) (Transformation|GetActorLocation) "0, 0, 0" 1.0 1.0 0.0 0 0 0)
  (Variables|Default|SetbPickedUp true)
  (CallFunction|Pickup(Server)))

(fn Drop
  (bind _staticmesh (Variables|Default|GetStaticMesh))
  (Physics|SetSimulatePhysics _staticmesh true)
  (Collision|SetCollisionEnabled _staticmesh "QueryAndPhysics")
  (Variables|Default|SetbPickedUp false))

(fn Use)

(fn SetObjectPosition)

(fn PrintLines
  (params (String%20to%20Print :type String) (Print%20Color :type Linear%20Color%20Structure :default "(R=1.000000,G=1.000000,B=1.000000,A=1.000000)") (String%20Duration :type Float%20%28single-precision%29))
  (if (Variables|Default|GetbPrint)
    (Development|PrintString String%20to%20Print true true Print%20Color String%20Duration)))