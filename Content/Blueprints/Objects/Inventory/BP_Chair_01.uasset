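; BP_Chair_01 is a carryable chair that the player uses to barricade doors.
; Use traces from the camera for an undestroyed BP_DoorBase without two chairs, closing it first if open.
; BlockDoor drops the chair, disables physics, attaches it front or back based on door Side, and registers it in ChairsBlocking.
; Pickup unregisters it from a locked door, while Tick detaches and launches it when the blocked door is destroyed.
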(event EventBeginPlay
  (|CallParentFunction) ; This node is disabled and will not be called.\nDrag off pins to build functionality.
)

(event Collision|EventActorBeginOverlap
  (params (OtherActor :type Actor%20Object%20Reference))
  (|CallParentFunction OtherActor) ; This node is disabled and will not be called.\nDrag off pins to build functionality.
)

(event EventTick
  (params (DeltaSeconds :type Float%20%28single-precision%29))
  (bind _door_to_block (Variables|Default|GetDoor%20To%20Block))
  (bind _staticmesh (Variables|Default|GetStaticMesh))
  (|CallParentFunction DeltaSeconds)
  (Utilities|IsValid _door_to_block
    (:Is%20Valid
      (if (and (Variables|Default|GetbBlocked) (Variables|/Game/Blueprints/Objects/Doors/BP_DoorBase.BP_DoorBase_C|GetbDestroyed _door_to_block))
        (Physics|SetSimulatePhysics _staticmesh true)
        (Physics|AddImpulseatLocation _staticmesh (* (Transformation|GetActorForwardVector) 2e+02) (Transformation|GetActorLocation) "None")
        (Transformation|DetachFromComponent (Variables|Default|GetStaticMesh) "KeepWorld" "KeepWorld" "KeepWorld" true)))))

(event EventSetObjectPosition
  (bind _asbp_player (Utilities|Casting|CastToBP_Player (Game|GetPlayerCharacter 0)))
  (Variables|Default|SetPosition (Variables|/Game/Characters/Player/BP_Player.BP_Player_C|GetChair _asbp_player)))

(event EventUse
  (bind _returnvalue (CallFunction|GetPlayer))
  (bind _camera (Variables|/Game/Characters/Player/BP_Player.BP_Player_C|GetCamera _returnvalue))
  (bind _returnvalue_2 (Transformation|GetWorldLocation _camera))
  (bind (_outhit _returnvalue_3) (Collision|LineTraceByChannel _returnvalue_2 (+ _returnvalue_2 (* (Math|Vector|GetForwardVector _camera) 2.4e+02)) "TraceTypeQuery1" false 0 "None"))
  (if _returnvalue_3
    (bind _asbp_door_base (Utilities|Casting|CastToBP_DoorBase (.HitActor (Collision|BreakHitResult _outhit))))
    (if (not (Variables|/Game/Blueprints/Objects/Doors/BP_DoorBase.BP_DoorBase_C|GetbDestroyed _asbp_door_base))
      (if (not (== (Utilities|Array|Length (Variables|/Game/Blueprints/Objects/Doors/BP_DoorBase.BP_DoorBase_C|GetChairs%20Blocking _asbp_door_base)) 2))
        (bind _output_get (Variables|Default|SetDoor%20To%20Block _asbp_door_base))
        (if (not (and (Variables|/Game/Blueprints/Objects/Doors/BP_DoorBase.BP_DoorBase_C|GetbLocked _output_get) (Variables|Default|GetbBlocked)))
          (if (Variables|/Game/Blueprints/Objects/Doors/BP_DoorBase.BP_DoorBase_C|GetbClosed (Variables|Default|GetDoor%20To%20Block))
            (CallFunction|BlockDoor)
            (else
              (Default|Close (Variables|Default|GetDoor%20To%20Block))
              (Utilities|FlowControl|Delay (/ 1.0 (Variables|/Game/Blueprints/Objects/Doors/BP_DoorBase.BP_DoorBase_C|GetSpeed (Variables|Default|GetDoor%20To%20Block))))
              (CallFunction|BlockDoor))))))))

(fn ConstructionScript
  (|CallParentFunction))

(fn Pickup
  (|CallParentFunction)
  (Utilities|IsValid (Variables|Default|GetDoor%20To%20Block)
    (:Is%20Valid
      (if (and (Variables|/Game/Blueprints/Objects/Doors/BP_DoorBase.BP_DoorBase_C|GetbLocked (Variables|Default|GetDoor%20To%20Block)) (Variables|Default|GetbBlocked))
        (Utilities|Array|RemoveItem (Variables|/Game/Blueprints/Objects/Doors/BP_DoorBase.BP_DoorBase_C|GetChairs%20Blocking (Variables|Default|GetDoor%20To%20Block)) self)
        (Variables|Default|SetbBlocked false)))))

(fn BlockDoor
  (bind _door_to_block (Variables|Default|GetDoor%20To%20Block))
  (bind _side (Variables|/Game/Blueprints/Objects/Doors/BP_DoorBase.BP_DoorBase_C|GetSide _door_to_block))
  (CallFunction|Drop)
  (Default|Drop(Event) (CallFunction|GetPlayer))
  (Physics|SetSimulatePhysics (Variables|Default|GetStaticMesh) false)
  (if (<= _side -0.1)
    (Transformation|AttachComponentToComponent self (Variables|/Game/Blueprints/Objects/Doors/BP_DoorBase.BP_DoorBase_C|GetChair_Front (Variables|Default|GetDoor%20To%20Block)) "None" "SnapToTarget" "SnapToTarget" "KeepRelative" true)
    (Utilities|Array|Add (Variables|/Game/Blueprints/Objects/Doors/BP_DoorBase.BP_DoorBase_C|GetChairs%20Blocking (Variables|Default|GetDoor%20To%20Block)) self)
    (Variables|Default|SetbBlocked true)
    (elif (>= _side -0.01)
      (Transformation|AttachComponentToComponent self (Variables|/Game/Blueprints/Objects/Doors/BP_DoorBase.BP_DoorBase_C|GetChair_Back (Variables|Default|GetDoor%20To%20Block)) "None" "SnapToTarget" "SnapToTarget" "KeepRelative" true)
      (Utilities|Array|Add (Variables|/Game/Blueprints/Objects/Doors/BP_DoorBase.BP_DoorBase_C|GetChairs%20Blocking (Variables|Default|GetDoor%20To%20Block)) self)
      (Variables|Default|SetbBlocked true))))