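; BP_Train is a practice train actor that moves its Cube component along the spline of a referenced Track, starting on BeginPlay.
; A timeline, optionally looping, plays at the inverse of LocomotiveSpeed, so that value scales travel duration rather than velocity.
; Each update converts timeline progress into a distance along the spline and sets the cube's world location and rotation from it, preserving scale.
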(event Custom|Follow%20Track
  ;[0.2758 0.4005 1] Follow Track
  (Utilities|IsValid (Variables|Default|GetTrack)
    (:Is%20Valid
      (Components|Timeline|SetLooping (Variables|Default|GetTL_Follow) (Variables|Default|GetbLoop))
      (Components|Timeline|SetPlayRate (Variables|Default|GetTL_Follow) (/ 1.0 (Variables|Default|GetLocomotive%20Speed)))
      (bind _location (Timeline|TL_Follow PlayFromStart)
        (:Update
          (bind _track (Variables|Default|GetTrack)
            (:then
              (Transformation|SetWorldTransform (Variables|Default|GetCube) (Math|Transform|MakeTransform (Spline|GetLocationatDistanceAlongSpline (Variables|/Game/PracticeFolder/BlueprintsPractice/BP_TrainSpline.BP_TrainSpline_C|GetSpline _track) (* _location (Spline|GetSplineLength (Variables|/Game/PracticeFolder/BlueprintsPractice/BP_TrainSpline.BP_TrainSpline_C|GetSpline _track))) "World") (Spline|GetRotationatDistanceAlongSpline (Variables|/Game/PracticeFolder/BlueprintsPractice/BP_TrainSpline.BP_TrainSpline_C|GetSpline _track) (* _location (Spline|GetSplineLength (Variables|/Game/PracticeFolder/BlueprintsPractice/BP_TrainSpline.BP_TrainSpline_C|GetSpline _track))) "World") (Transformation|GetWorldScale (Variables|Default|GetCube))) false false))
            (:else)))))))

(event EventBeginPlay
  ;[0.2758 0.4005 1] Begin Play
  (CallFunction|FollowTrack))

(fn ConstructionScript)