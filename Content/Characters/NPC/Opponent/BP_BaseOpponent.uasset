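; BP_BaseOpponent is a base NPC opponent with a hunger need, feeding its state to an AI blackboard.
; A looping timer drains Hunger, updates bHungry, and at zero enables mesh physics simulation and stops walking.
; AI perception updates bCanSeePlayer when sensing BP_Player.
; Helper functions replenish hunger, switch walk/run speed, print messages and step through BP_FoodBase actors by an incrementing, unchecked index.
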(event OnTargetPerceptionUpdated(AIPerception)
  (params (Actor :type Actor%20Object%20Reference) (Stimulus :type AI%20Stimulus%20Structure))
  ;[1 0.03646 0.03646] Set Can See Player
  (Utilities|Casting|CastToBP_Player Actor)
  (AI|Components|Blackboard|SetValueasBool (AI|GetBlackboard 0) (Utilities|Name|MakeLiteralName "bCanSeePlayer") (.bSuccessfullySensed (Utilities|Struct|BreakAIStimulus Stimulus))))

(event Custom|Check%20If%20Hungry
  ;[1 0.03646 0.03646] Check If Hungry
  (Health/Energy|DrainHunger 5.0)
  (AI|Components|Blackboard|SetValueasBool (AI|GetBlackboard 0) (Utilities|Name|MakeLiteralName "bHungry") (Health/Energy|IsHungry))
  (if (<= (Variables|Health/Energy|GetHunger) 0.0)
    (Physics|SetSimulatePhysics (Variables|Character|GetMesh) true)
    (Variables|/Script/Engine.CharacterMovementComponent|SetMaxWalkSpeed (Variables|Character|GetCharacterMovement) 0.0)))

(event EventBeginPlay
  ;[1 0.03646 0.03646] Begin Play
  (Utilities|Time|SetTimerbyEvent (delegate Custom|Check%20If%20Hungry) 3.0 true))

(fn ConstructionScript)

(fn SetWalkingSpeed
  (params (bRunning :type Boolean))
  (Variables|/Script/Engine.CharacterMovementComponent|SetMaxWalkSpeed (Variables|Character|GetCharacterMovement) (select bRunning (Variables|CharacterSpeeds|GetRunning) (Variables|CharacterSpeeds|GetWalking))))

(fn PrintLines
  (params (String%20To%20Print :type String) (String%20Color :type Linear%20Color%20Structure :default "(R=1.000000,G=1.000000,B=1.000000,A=1.000000)") (String%20Duration :type Float%20%28single-precision%29))
  (Development|PrintString String%20To%20Print true true String%20Color String%20Duration))

(fn ReplenishHunger
  (params (Amount%20To%20Replenish :type Float%20%28single-precision%29))
  (Variables|Health/Energy|SetHunger (+ (Variables|Health/Energy|GetHunger) Amount%20To%20Replenish)))

(fn SearchforFood
  (bind _outactors (Actor|GetAllActorsOfClass "/Game/Blueprints/Objects/Food/BP_FoodBase.BP_FoodBase_C"))
  (Math|Integer|IncrementInt (LocalVariables|GetFood%20Index)
    (:%20%20
      (return (Utilities|Array|Get(acopy) _outactors (LocalVariables|GetFood%20Index))))))

(fn DrainHunger
  (params (Hunger%20To%20Drain :type Float%20%28single-precision%29))
  (Variables|Health/Energy|SetHunger (- (Variables|Health/Energy|GetHunger) Hunger%20To%20Drain)))

(fn IsHungry
  (return (<= (Variables|Health/Energy|GetHunger) 25.0)))