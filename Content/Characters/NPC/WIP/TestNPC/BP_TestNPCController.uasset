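; AI controller for the work-in-progress test NPC that runs the BT_TestNPC behavior tree on BeginPlay.
; After starting the tree, it adds a Blackboard component and caches it along with the controlled BP_TestNPC pawn.
; Each Tick writes the inverse of the pawn's CanSeePlayer flag to the bCanSeePlayer blackboard key, so the key's value is opposite to its name.
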(event EventBeginPlay
  (AI|RunBehaviorTree "/Game/Characters/NPC/WIP/TestNPC/AI/Behavior/BT_TestNPC.BT_TestNPC")
  (bind _returnvalue (AddComponent|AddBlackboardComponent))
  (Variables|Default|SetBB _returnvalue)
  (bind _asbp_test_npc (Utilities|Casting|CastToBP_TestNPC (Pawn|GetControlledPawn)))
  (Variables|Default|SetNPC _asbp_test_npc))

(event EventTick
  (params (DeltaSeconds :type Float%20%28single-precision%29))
  (AI|Components|Blackboard|SetValueasBool (Variables|Default|GetBB) (Utilities|Name|MakeLiteralName "bCanSeePlayer") (not (Variables|/Game/Characters/NPC/WIP/TestNPC/BP_TestNPC.BP_TestNPC_C|GetbCanSeePlayer (Variables|Default|GetNPC)))))

(fn ConstructionScript)