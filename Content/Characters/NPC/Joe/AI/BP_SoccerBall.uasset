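; BP_SoccerBall is a kickable ball actor that the player interacts with and that works with BP_Goal for scoring.
; Interact applies a random-strength impulse along the player's forward vector, with sound, particles and a short DoOnce cooldown.
; BallKicked plays effects and increments AIPoints on the first BP_Goal found, while BallWentThroughGoal restores the transform saved at BeginPlay.
; Server-to-multicast Open events relay InteractMessage, and a Debug flag shows an arrow.
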(event Custom|Open%20%28Server%29
  (params (Actor :type Object%20Object%20Reference) (Component :type Scene%20Component%20Object%20Reference))
  ;[1 0.03646 0.03646] Replicated Events
  (CallFunction|Open(Multicast) Actor Component))

(event Custom|Open%20%28Multicast%29
  (params (Actor :type Object%20Object%20Reference) (Component :type Scene%20Component%20Object%20Reference))
  ;[1 0.03646 0.03646] Replicated Events
  (Class|BPIInteraction|Interact(Message) Actor Component))

(event Custom|CustomEvent_1
  ;[0.4601 0.3281 1] Begin Play
  (bind _asbp_player (Utilities|Casting|CastToBP_Player (Game|GetPlayerCharacter 0)))
  (Variables|Default|SetPlayer _asbp_player))

(event EventTick
  (params (DeltaSeconds :type Float%20%28single-precision%29))
  ;[0.4601 0.3281 1] Tick
)

(event EventBeginPlay
  ;[0.9686 0.2941 1] Begin Play
  (bind _asbp_player (Utilities|Casting|CastToBP_Player (Game|GetPlayerCharacter 0)))
  (Variables|Default|SetPlayer _asbp_player)
  (Variables|Default|SetOriginal%20Transform (Transformation|GetWorldTransform (Variables|Default|GetSphere))))

(event EventInteract
  (params (Component :type Scene%20Component%20Object%20Reference))
  (bind _returnvalue (Transformation|GetActorLocation))
  ;[0.9686 0.2941 1] Kick Ball
  (Utilities|FlowControl|DoOnce false :!label _label
    (:Completed
      (Physics|AddImpulseatLocation (Variables|Default|GetSphere) (* (Math|Vector|GetForwardVector (Variables|/Script/Engine.Actor|GetRootComponent (Variables|Default|GetPlayer))) (Math|Random|RandomFloatinRange 4e+04 8e+04)) _returnvalue "None")
      (Audio|SpawnSoundatLocation "/Game/Audio/SFX/Characters/Joe/CUE_BallKick.CUE_BallKick" (Variables|/Script/Engine.SceneComponent|GetRelativeLocation (Variables|Default|GetSphere)) "0, 0, 0" 1.0 1.0 0.0 0 0)
      (Effects|SpawnEmitterAttached "/Game/Effects/Particles/Cascade/P_SoccerBallImpact.P_SoccerBallImpact" (Variables|Default|GetSphere) "None" _returnvalue)
      (Utilities|FlowControl|Delay 0.1)
      (goto _label Reset))))

(fn ConstructionScript
  (bind _arrow (Variables|Default|GetArrow))
  (if (Variables|Default|GetbDebug)
    (Development|SetHiddeninGame _arrow false false)
    (else
      (Development|SetHiddeninGame _arrow true false))))

(fn BallKicked
  (bind _returnvalue (Transformation|GetActorLocation))
  (Audio|SpawnSoundatLocation "/Game/Audio/SFX/Characters/Joe/CUE_BallKick.CUE_BallKick" _returnvalue "0, 0, 0" 1.0 1.0 0.0 0 0)
  (Effects|SpawnEmitteratLocation "/Game/Effects/Particles/Cascade/P_SoccerBallImpact.P_SoccerBallImpact" _returnvalue)
  (bind _outactors (Actor|GetAllActorsOfClass "/Game/Characters/NPC/Joe/AI/BP_Goal.BP_Goal_C"))
  (Math|Integer|IncrementInt (Variables|/Game/Characters/NPC/Joe/AI/BP_Goal.BP_Goal_C|GetAI%20Points (Utilities|Array|Get(acopy) _outactors))))

(fn BallWentThroughGoal
  (Transformation|SetActorRelativeTransform (Variables|Default|GetOriginal%20Transform) false false))