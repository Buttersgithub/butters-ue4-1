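; BP_Goal is a soccer goal that scores for the player when a BP_SoccerBall overlaps its box.
; A DoOnce-gated timeline animates a light flash, then increments PlayerPoints, destroys the ball and spawns another at the player's transform.
; The gate resets through a delay fired from the timeline's update.
; CheckPoints, uncalled here, sends taunts to the soccer UI of the cached BP_Joe based on AIPoints.
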(event OnComponentBeginOverlap(Box)
  (params (OverlappedComponent :type Primitive%20Component%20Object%20Reference) (OtherActor :type Actor%20Object%20Reference) (OtherComp :type Primitive%20Component%20Object%20Reference) (OtherBodyIndex :type Integer) (bFromSweep :type Boolean) (SweepResult :type Hit%20Result%20Structure%20%28by%20ref%29))
  ;[0.1996 0.3151 1] Overlap
  (bind _asbp_soccer_ball (Utilities|Casting|CastToBP_SoccerBall OtherActor))
  (Variables|Default|SetBall _asbp_soccer_ball)
  (Utilities|FlowControl|DoOnce false :!label _label
    (:Completed
      (bind _light (Timeline|TL_Victory PlayFromStart)
        (:Update
          (Rendering|Components|Light|SetIntensity (Variables|Default|GetPointLight) (Math|Float|Lerp 0.0 5e+03 _light))
          (Utilities|FlowControl|Delay 2.0)
          (goto _label Reset))
        (:Finished
          (Math|Integer|IncrementInt (Variables|Default|GetPlayer%20Points)
            (:%20%20
              (Actor|DestroyActor (Variables|Default|GetBall))
              (Game|SpawnActorfromClass "/Game/Characters/NPC/Joe/AI/BP_SoccerBall.BP_SoccerBall_C" (Transformation|GetActorTransform (Game|GetPlayerCharacter 0)) "Undefined" 0 0))))))))

(event EventBeginPlay
  ;[0.1996 0.3151 1] Begin Play
  (CallFunction|CreateJoeReference)
  (bind _outactors (Actor|GetAllActorsOfClass "/Game/Characters/NPC/Joe/AI/BP_SoccerBall.BP_SoccerBall_C"))
  (Variables|Default|SetBall (Utilities|Array|Get(acopy) _outactors)))

(fn ConstructionScript)

(fn CreateJoeReference
  (bind _outactors (Actor|GetAllActorsOfClass "/Game/Characters/NPC/Joe/BP_Joe.BP_Joe_C"))
  (Variables|Default|SetJoe (Utilities|Array|Get(acopy) _outactors)))

(fn CheckPoints
  (switch int (Variables|Default|GetAI%20Points)
    (:0
      (Default|SendMessage (Variables|/Game/Characters/NPC/Joe/BP_Joe.BP_Joe_C|GetSoccer%20UI (Variables|Default|GetJoe)) "You suck."))
    (:1
      (Default|SendMessage (Variables|/Game/Characters/NPC/Joe/BP_Joe.BP_Joe_C|GetSoccer%20UI (Variables|Default|GetJoe)) "Get better."))
    (:2
      (Default|SendMessage (Variables|/Game/Characters/NPC/Joe/BP_Joe.BP_Joe_C|GetSoccer%20UI (Variables|Default|GetJoe)) "You are honestly terrible."))
    (:3
      (Default|SendMessage (Variables|/Game/Characters/NPC/Joe/BP_Joe.BP_Joe_C|GetSoccer%20UI (Variables|Default|GetJoe)) "Are you even trying at this point?"))
    (:4
      (Default|SendMessage (Variables|/Game/Characters/NPC/Joe/BP_Joe.BP_Joe_C|GetSoccer%20UI (Variables|Default|GetJoe)) "Bro.."))
    (:5
      (Default|SendMessage (Variables|/Game/Characters/NPC/Joe/BP_Joe.BP_Joe_C|GetSoccer%20UI (Variables|Default|GetJoe)) "Please get better. this is boring."))))