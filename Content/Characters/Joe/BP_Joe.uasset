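; BP_Joe is a soccer character that moves its mesh along a sideways line and kicks any soccer ball within reach.
; A timeline started on BeginPlay lerps the mesh's relative location, with play rate set by MovementSpeed.
; Detection sphere overlaps track the ball, and Tick applies an impulse along the ball's arrow and calls BallKicked, with a DoOnce-and-delay cooldown.
; The construction script sets detection radius and debug visibility.
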(event OnComponentBeginOverlap(BallDetection)
  (params (OverlappedComponent :type Primitive%20Component%20Object%20Reference) (OtherActor :type Actor%20Object%20Reference) (OtherComp :type Primitive%20Component%20Object%20Reference) (OtherBodyIndex :type Integer) (bFromSweep :type Boolean) (SweepResult :type Hit%20Result%20Structure%20%28by%20ref%29))
  ;[0.8919 0.3575 1] Check if the ball is in the Detection Sphere
  (bind _asbp_soccer_ball (Utilities|Casting|CastToBP_SoccerBall OtherActor))
  (Variables|Default|SetBall _asbp_soccer_ball)
  (Variables|Default|SetbBallInDetectionSphere true))

(event OnComponentEndOverlap(BallDetection)
  (params (OverlappedComponent :type Primitive%20Component%20Object%20Reference) (OtherActor :type Actor%20Object%20Reference) (OtherComp :type Primitive%20Component%20Object%20Reference) (OtherBodyIndex :type Integer))
  ;[0.8919 0.3575 1] Check if the ball is in the Detection Sphere
  (bind _asbp_soccer_ball (Utilities|Casting|CastToBP_SoccerBall OtherActor))
  (Variables|Default|SetBall _asbp_soccer_ball)
  (Variables|Default|SetbBallInDetectionSphere false))

(event EventTick
  (params (DeltaSeconds :type Float%20%28single-precision%29))
  (bind _ball (Variables|Default|GetBall))
  ;[0.8919 0.3575 1] Tick
  (if (Variables|Default|GetbBallInDetectionSphere)
    (Utilities|FlowControl|DoOnce false :!label _label
      (:Completed
        (Utilities|Casting|CastToBP_Player (Game|GetPlayerCharacter 0))
        (Physics|AddImpulseatLocation (Variables|/Game/Characters/Joe/AI/BP_SoccerBall.BP_SoccerBall_C|GetSphere _ball) (* (Math|Vector|GetForwardVector (Variables|/Game/Characters/Joe/AI/BP_SoccerBall.BP_SoccerBall_C|GetArrow _ball)) (Variables|Default|GetBall%20Kick%20Force)) (Transformation|GetActorLocation _ball) "None")
        (Default|BallKicked _ball)
        (Utilities|FlowControl|Delay 2.0)
        (goto _label Reset)))))

(event EventBeginPlay
  ;[0.8919 0.3575 1] Move Character
  (Components|Timeline|SetPlayRate (Variables|Default|GetTL_Move) (/ (Variables|Default|GetMovement%20Speed) 1.0))
  (bind _location (Timeline|TL_Move Play)
    (:Update
      (Transformation|SetRelativeLocation (Variables|Character|GetMesh) (Math|Vector|Lerp(Vector) "0, 0, 0" "0,500.000000, 0" _location) false false))))

(fn ConstructionScript
  (bind _ball_detection (Variables|Default|GetBall%20Detection))
  (Utilities|FlowControl|Sequence
    (:then_0
      (if (Variables|Default|GetbDebug)
        (Development|SetHiddeninGame _ball_detection false false)
        (else
          (Development|SetHiddeninGame _ball_detection true false))))
    (:then_1
      (Components|Sphere|SetSphereRadius (Variables|Default|GetBall%20Detection) (Variables|Default|GetDetection%20Radius) true))))