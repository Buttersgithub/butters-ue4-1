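; BP_ButtersGameInstance is the game instance that handles hosting and joining multiplayer sessions through Advanced Sessions nodes.
; HostSession creates a session tagged with a server name built from the player's name, then opens the landscape test level on success.
; JoinSession joins the supplied search result.
; Both success paths switch the first player controller to game-only input, and neither event handles failure.
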(event Custom|Host%20Session
  (params (Player%20Name :type Text))
  (|AdvancedSession (Utilities|Array|MakeArray (Class|AdvancedSessionsLibrary|MakeLiteralSessionPropertyString "SNAME" (Utilities|String|Append (Utilities|String|ToString(Text) Player%20Name) "'s " "Server"))) (Game|GetPlayerController 0) 100 0 false true false true true true false false false true
    (:OnSuccess
      (Input|SetInputModeGameOnly (Game|GetPlayerController 0))
      (Game|OpenLevel(byName) "LVL_LandscapeTest_01" true "?listen"))))

(event Custom|Join%20Session
  (params (Session :type Blueprint%20Session%20Result%20Structure))
  (|JoinSession (Game|GetPlayerController 0) Session
    (:OnSuccess
      (Input|SetInputModeGameOnly (Game|GetPlayerController 0)))))