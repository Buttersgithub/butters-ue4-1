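; BP_Water is a placeable water plane whose look is chosen through its WaterType and WaterSize settings.
; The construction script sets the Plane material to the standard water instance by default, or to a cartoon water instance for the Cartoony type.
; For Cartoony water, a second pass picks the Small or Big material variant.
; The event graph holds no active logic.
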(event EventBeginPlay)

(event Collision|EventActorBeginOverlap
  (params (OtherActor :type Actor%20Object%20Reference)))

(event EventTick
  (params (DeltaSeconds :type Float%20%28single-precision%29)))

(fn ConstructionScript
  (bind _plane (Variables|Default|GetPlane))
  (bind _plane_2 (Variables|Default|GetPlane))
  (Utilities|FlowControl|Sequence
    (:then_0
      (switch Utilities|FlowControl|Switch|SwitchonENUM_WaterType (Variables|Default|GetWater%20Type)
        (:NewEnumerator0
          (Rendering|Material|SetMaterial _plane_2 0 "/Game/Effects/Water/Default/MI_Water_01.MI_Water_01"))
        (:NewEnumerator1
          (Rendering|Material|SetMaterial _plane_2 0 "/Game/Effects/Water/Cartoony/MI_CartoonWater_01.MI_CartoonWater_01"))))
    (:then_1
      (if (Utilities|Enum|Equal(Enum) (Variables|Default|GetWater%20Type) "NewEnumerator1")
        (switch Utilities|FlowControl|Switch|SwitchonENUM_WaterSize (Variables|Default|GetWater%20Size)
          (:NewEnumerator0
            (Rendering|Material|SetMaterial _plane 0 "/Game/Effects/Water/Cartoony/MI_CartoonWater_01.MI_CartoonWater_01"))
          (:NewEnumerator1
            (Rendering|Material|SetMaterial _plane 0 "/Game/Effects/Water/Cartoony/MI_CartoonWater_02.MI_CartoonWater_02")))))))