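; BP_Locomotive is a train vehicle that rides a BP_TrainTrackSpline, shoving players it hits and sounding a horn when they enter its trigger.
; On BeginPlay a server event multicasts the follow logic, where a timeline scaled by LocomotiveSpeed moves the mesh along the spline, optionally looping.
; Overlaps launch players along the arrow or play the horn, each with a reset cooldown.
; Helper functions attach it to the nearest track or restore its original transform.
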(event OnComponentBeginOverlap(Box)
  (params (OverlappedComponent :type Primitive%20Component%20Object%20Reference) (OtherActor :type Actor%20Object%20Reference) (OtherComp :type Primitive%20Component%20Object%20Reference) (OtherBodyIndex :type Integer) (bFromSweep :type Boolean) (SweepResult :type Hit%20Result%20Structure%20%28by%20ref%29))
  ;[0.2758 0.4005 1] Overlapping
  (bind _asbp_player (Utilities|Casting|CastToBP_Player OtherActor))
  (Utilities|FlowControl|DoOnce false :!label _label
    (:Completed
      (Character|LaunchCharacter _asbp_player (* (Math|Vector|GetForwardVector (Variables|Default|GetArrow)) (Variables|LocomotiveSettings|GetPlayer%20Push%20Force)) false false)
      (Utilities|FlowControl|Delay 1.0)
      (goto _label Reset))))

(event OnComponentBeginOverlap(LocomotiveHornTrigger)
  (params (OverlappedComponent :type Primitive%20Component%20Object%20Reference) (OtherActor :type Actor%20Object%20Reference) (OtherComp :type Primitive%20Component%20Object%20Reference) (OtherBodyIndex :type Integer) (bFromSweep :type Boolean) (SweepResult :type Hit%20Result%20Structure%20%28by%20ref%29))
  ;[0.2758 0.4005 1] Horn Sounds
  (Utilities|Casting|CastToBP_Player OtherActor)
  (Utilities|FlowControl|DoOnce false :!label _label
    (:Completed
      (Audio|Components|Audio|Play (Variables|Default|GetCUE_LocomotiveHorn) 0.0)
      (Utilities|FlowControl|Delay 4.0)
      (goto _label Reset))))

(event Custom|Follow%20Track%20%28Server%29
  ;[0.2758 0.4005 1] Follow Track
  (CallFunction|FollowTrack(Multicast)))

(event Custom|Follow%20Track%20%28Multicast%29
  ;[0.2758 0.4005 1] Follow Track
  (Utilities|IsValid (Variables|References|GetTrack)
    (:Is%20Valid
      (Components|Timeline|SetLooping (Variables|Default|GetTL_Follow) (Variables|LocomotiveSettings|GetbLoop))
      (Components|Timeline|SetPlayRate (Variables|Default|GetTL_Follow) (/ 1.0 (Math|Conversions|ToFloat(Integer) (Variables|LocomotiveSettings|GetLocomotive%20Speed))))
      (bind _location (Timeline|TL_Follow PlayFromStart)
        (:Update
          (bind _track (Variables|References|GetTrack)
            (:then
              (Transformation|SetWorldTransform (Variables|Default|GetStaticMesh) (Math|Transform|MakeTransform (Spline|GetLocationatDistanceAlongSpline (Variables|/Game/GameplayLogic/Locomotive/BP_TrainTrackSpline.BP_TrainTrackSpline_C|GetSpline _track) (* _location (Spline|GetSplineLength (Variables|/Game/GameplayLogic/Locomotive/BP_TrainTrackSpline.BP_TrainTrackSpline_C|GetSpline _track))) "World") (Spline|GetRotationatDistanceAlongSpline (Variables|/Game/GameplayLogic/Locomotive/BP_TrainTrackSpline.BP_TrainTrackSpline_C|GetSpline _track) (* _location (Spline|GetSplineLength (Variables|/Game/GameplayLogic/Locomotive/BP_TrainTrackSpline.BP_TrainTrackSpline_C|GetSpline _track))) "World") (Transformation|GetWorldScale (Variables|Default|GetStaticMesh))) false false)
              (if (Variables|Default|GetbDebug)
                (Rendering|Debug|DrawDebugArrow (Transformation|GetActorLocation) (Spline|GetLocationatDistanceAlongSpline (Variables|/Game/GameplayLogic/Locomotive/BP_TrainTrackSpline.BP_TrainTrackSpline_C|GetSpline _track) (* _location (Spline|GetSplineLength (Variables|/Game/GameplayLogic/Locomotive/BP_TrainTrackSpline.BP_TrainTrackSpline_C|GetSpline _track))) "World") 1e+01 "(R=1.000000,G=0.000000,B=0.000000,A=1.000000)" 0.0 25.0)))
            (:else)))))))

(event EventBeginPlay
  ;[0.2758 0.4005 1] Begin Play
  (Utilities|IsValid (Variables|References|GetTrack)
    (:Is%20Valid
      (CallFunction|FollowTrack(Server)))))

(fn ConstructionScript
  (Components|StaticMesh|SetStaticMesh (Variables|Default|GetStaticMesh) (Variables|LocomotiveSettings|GetCarriage%20Mesh))
  (Variables|LocomotiveSettings|SetLocomotive%20Speed (Variables|LocomotiveSettings|GetLocomotive%20Speed))
  (Transformation|SetWorldRotation (Variables|Default|GetLocomotiveHornTrigger) "0, 0, 0" false false))

(fn PlaceonNearestTrack
  (bind _returnvalue (Transformation|GetActorTransform))
  (Utilities|IsValid (Variables|References|GetTrack)
    (:Is%20Not%20Valid
      (Variables|LocomotiveSettings|SetLocomotive%20Original%20Transform (Math|Transform|MakeTransform (.location _returnvalue) (.rotation _returnvalue) (Transformation|GetActorScale3D)))
      (bind _nearest_actor (CallFunction|GetNearestActorOfClass "/Game/GameplayLogic/Locomotive/BP_TrainTrackSpline.BP_TrainTrackSpline_C" (Transformation|GetActorLocation)))
      (bind _asbp_train_track_spline (Utilities|Casting|CastToBP_TrainTrackSpline _nearest_actor))
      (bind _output_get (Variables|References|SetTrack _asbp_train_track_spline))
      (Utilities|IsValid _output_get
        (:Is%20Valid
          (Transformation|SetActorLocationAndRotation (Transformation|GetActorLocation _output_get) (Transformation|GetActorRotation _output_get)))))))

(fn RemovefromCurrentTrack
  (Variables|References|GetTrack
    (:then
      (Variables|References|SetTrack 0)
      (Transformation|SetActorTransform (Variables|LocomotiveSettings|GetLocomotive%20Original%20Transform)))
    (:else)))