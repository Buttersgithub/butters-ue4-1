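; BP_ButtersFunctionLibrary is a function library of shared gameplay helpers for actor queries, game mode and player access, and math.
; Actor searches return exact-class matches or the actor nearest to a location.
; GetPlayer uses the player stored on BP_InGameGameMode, falling back to the player character, then a world search.
; Math helpers lerp 2D vectors, combine transforms keeping the first scale, and solve launch velocity for a timed arc under hardcoded gravity.
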(fn GetAllActorsOfSpecificClass
  (params (Class :type Actor%20Class%20Reference))
  (bind _outactors (Actor|GetAllActorsOfClass 0 "/Script/Engine.Actor"))
  (for _array_element _outactors
    (if (== (Utilities|GetClass _array_element) Class)
      (Utilities|Array|AddUnique (LocalVariables|GetReturned%20Value) _array_element)))
  (return (LocalVariables|GetReturned%20Value)))

(fn GetNearestActorOfClass
  (params (Class :type Actor%20Class%20Reference) (Class%20Location :type Vector))
  (bind _outactors (Actor|GetAllActorsOfClass 0 Class))
  (for _array_element _outactors
    (if (< (Math|Vector|Distance(Vector) (Transformation|GetActorLocation _array_element) Class%20Location) (LocalVariables|GetLV_Nearest%20Distance))
      (LocalVariables|SetLV_Nearest%20Distance (Math|Vector|Distance(Vector) (Transformation|GetActorLocation _array_element) Class%20Location))
      (LocalVariables|SetLV_Nearest%20Actor _array_element)))
  (return (LocalVariables|GetLV_Nearest%20Actor) (LocalVariables|GetLV_Nearest%20Distance)))

(fn GetButtersGameMode
  (bind _asbp_in_game_game_mode (Utilities|Casting|CastToBP_InGameGameMode (Game|GetGameMode (LocalVariables|Get__WorldContext)))
    (:then
      (return _asbp_in_game_game_mode))
    (:CastFailed
      (return 0))))

(fn Lerp(Vector2D)
  (params (A :type Vector%202D%20Structure) (B :type Vector%202D%20Structure) (Alpha :type Float%20%28single-precision%29))
  (bind (_x _y) (Math|Vector2D|BreakVector2D B))
  (bind (_x_2 _y_2) (Math|Vector2D|BreakVector2D A))
  (return (Math|Vector2D|MakeVector2D (Math|Float|Lerp _x_2 _x Alpha) (Math|Float|Lerp _y_2 _y Alpha))))

(fn AddTransform
  (params (A :type Transform) (B :type Transform))
  (bind (_location _rotation) (Math|Transform|BreakTransform B))
  (bind (_location_2 _rotation_2 _scale) (Math|Transform|BreakTransform A))
  (return (Math|Transform|MakeTransform (+ _location_2 _location) (Math|Rotator|CombineRotators _rotation_2 _rotation) _scale)))

(fn CalculateArc
  (params (A :type Vector) (B :type Vector) (Time :type Float%20%28single-precision%29))
  (bind (_x _y _z) (Math|Vector|BreakVector A))
  (bind (_x_2 _y_2 _z_2) (Math|Vector|BreakVector B))
  (return (Math|Vector|MakeVector (/ (- _x_2 _x) Time) (/ (- _y_2 _y) Time) (/ (- _z_2 (+ _z (* (Math|Float|Square Time) -0.5 982.0))) Time))))

(fn GetPlayer
  (bind ___worldcontext (LocalVariables|Get__WorldContext))
  (bind _returnvalue (CallFunction|GetButtersGameMode ___worldcontext))
  (bind _player (Variables|/Game/GameplayLogic/GameModes/BP_InGameGameMode.BP_InGameGameMode_C|GetPlayer _returnvalue))
  (Utilities|IsValid _player
    (:Is%20Valid
      (return _player (Transformation|GetActorLocation _player)))
    (:Is%20Not%20Valid
      (bind _asbp_player (Utilities|Casting|CastToBP_Player (Game|GetPlayerCharacter ___worldcontext))
        (:then
          (return _asbp_player (Transformation|GetActorLocation _asbp_player)))
        (:CastFailed
          (bind _returnvalue_2 (Actor|GetActorOfClass ___worldcontext "/Game/Characters/Player/BP_Player.BP_Player_C"))
          (return _returnvalue_2 (Transformation|GetActorLocation _returnvalue_2)))))))