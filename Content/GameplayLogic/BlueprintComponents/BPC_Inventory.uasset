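; BPC_Inventory is an inventory component that expects its owner to be a BP_ItemBase item.
; On BeginPlay it caches three references: the owning item, the BP_Player character at index 0, and the InventoryWidget held by BP_InGameGameMode.
; Its event graph contains only this setup, with no logic for adding, removing or using items.
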(event EventBeginPlay
  (Utilities|FlowControl|Sequence
    (:then_0
      (bind _asbp_item_base (Utilities|Casting|CastToBP_ItemBase (Components|GetOwner)))
      (Variables|Default|SetItem _asbp_item_base))
    (:then_1
      (bind _asbp_player (Utilities|Casting|CastToBP_Player (Game|GetPlayerCharacter 0)))
      (Variables|Default|SetPlayer _asbp_player))
    (:then_2
      (bind _asbp_in_game_game_mode (Utilities|Casting|CastToBP_InGameGameMode (Game|GetGameMode)))
      (Variables|Default|SetInventory%20Widget (Variables|/Game/GameplayLogic/GameModes/BP_InGameGameMode.BP_InGameGameMode_C|GetInventory%20Widget _asbp_in_game_game_mode)))))