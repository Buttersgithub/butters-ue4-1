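; BP_LobbyPlayer sets up the lobby screen for the local player when play begins.
; BeginPlay creates the WBP_Lobby widget for player controller 0, adds it to the viewport, switches input to UI only and shows the mouse cursor.
; When the Steam online subsystem is present, it passes a welcome text with the player's online nickname to the widget.
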(event EventBeginPlay
  (bind _returnvalue (UserInterface|CreateWidget "/Game/Blueprints/Widgets/Lobby/WBP_Lobby.WBP_Lobby_C" (Game|GetPlayerController 0)))
  (bind _output_get (Variables|Default|SetLobby _returnvalue))
  (UserInterface|Viewport|AddtoViewport _output_get 0)
  (Input|SetInputModeUIOnly (Game|GetPlayerController 0) _output_get "DoNotLock")
  (Utilities|IsValid (Widget|GetOwningPlayer _output_get)
    (:Is%20Valid
      (Variables|/Script/Engine.PlayerController|SetbShowMouseCursor (Widget|GetOwningPlayer _output_get) true)
      (if (Class|AdvancedSessionsLibrary|HasOnlineSubsystem "STEAM")
        (Default|UpdatePlayerName (Variables|Default|GetLobby) (Utilities|Text|ToText(String) (Utilities|String|Append "Welcome, " (Class|AdvancedIdentityLibrary|GetPlayerNickname (Class|AdvancedSessionsLibrary|GetUniqueNetID (Game|GetPlayerController 0))))))))))

(fn ConstructionScript)